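; BP_SpawnGrid is the grid spawner for the Game of Life, laying out BP_Cell actors at CellDistance spacing.
; On BeginPlay it adds WBP_Input to the viewport, spawns the default GridX by GridY grid and binds the widget's click event inside the spawn loop.
; A click destroys all existing cells and respawns the grid using the sizes typed into the widget.
; Both passes offset cell Y from the spawner's X location.
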(event `self.ReceiveBeginPlay`
  (bind (_returnvalue_x _returnvalue_y _returnvalue_z) (`KismetMathLibrary.BreakVector` (`self.K2_GetActorLocation`)))
  (bind _returnvalue (`|CreateWidget` "/Game/Blueprints/GameOfLifeBP/WBP_Input.WBP_Input_C" (`GameplayStatics.GetPlayerController` 0)))
  (bind _output_get (set `self.UIInput` _returnvalue))
  (`UserWidget.AddToViewport` _output_get 0)
  (for _index (range (+ (`self.GridY`) 1))
    (set `self.TempY` (* _index (`self.CellDistance`)))
    (for _index_2 (range (+ (`self.GridX`) 1))
      (`|SpawnActorFromClass` "/Game/Blueprints/GameOfLifeBP/BP_Cell.BP_Cell_C" (`KismetMathLibrary.MakeTransform` (`KismetMathLibrary.MakeVector` (`KismetMathLibrary.Conv_IntToDouble` (* _index_2 (`self.CellDistance`))) (+ _returnvalue_x (`self.TempY`)) _returnvalue_z)) "Undefined" "MultiplyWithRoot" null null)
      (add `/Game/Blueprints/GameOfLifeBP/WBP_Input.OnClickedTest` (`self.UIInput`) (delegate `ClickGenerateGrid`)))))

(event `ClickGenerateGrid`
  (bind (_returnvalue_x _returnvalue_y _returnvalue_z) (`KismetMathLibrary.BreakVector` (`self.K2_GetActorLocation`)))
  (bind _outactors (`GameplayStatics.GetAllActorsOfClass` "/Game/Blueprints/GameOfLifeBP/BP_Cell.BP_Cell_C"))
  (`self.K2_DestroyActor` _outactors)
  (for _index (range (+ (`KismetStringLibrary.Conv_StringToInt` (`KismetTextLibrary.Conv_TextToString` (`/Game/Blueprints/GameOfLifeBP/WBP_Input.GridYText` (`self.UIInput`)))) 1))
    (set `self.TempY` (* _index (`self.CellDistance`)))
    (for _index_2 (range (+ (`KismetStringLibrary.Conv_StringToInt` (`KismetTextLibrary.Conv_TextToString` (`/Game/Blueprints/GameOfLifeBP/WBP_Input.GridXText` (`self.UIInput`)))) 1))
      (`|SpawnActorFromClass` "/Game/Blueprints/GameOfLifeBP/BP_Cell.BP_Cell_C" (`KismetMathLibrary.MakeTransform` (`KismetMathLibrary.MakeVector` (`KismetMathLibrary.Conv_IntToDouble` (* _index_2 (`self.CellDistance`))) (+ _returnvalue_x (`self.TempY`)) _returnvalue_z)) "Undefined" "MultiplyWithRoot" null null))))

(fn `UserConstructionScript`)