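; Grid cell actor for a Game of Life simulation that starts randomly alive or dead.
; A looping timer fires eight rotated line traces, drawn persistently, adding living BP_Cell neighbours to a counter that is never reset.
; A count of two or three sets the cell alive regardless of its current state; otherwise it dies.
; Each state swaps dynamic materials and plays a timeline animating hue (alive) or value (dead).
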(event `self.ReceiveBeginPlay`
  (bind _cell (`self.Cell`))
  (bind _returnvalue (`PrimitiveComponent.CreateDynamicMaterialInstance` _cell 0 "/Game/Materials/M_CellDead.M_CellDead" "None"))
  (set `self.DeadMI` _returnvalue)
  (bind _returnvalue_2 (`PrimitiveComponent.CreateDynamicMaterialInstance` _cell 0 "/Game/Materials/M_CellAlive.M_CellAlive" "None"))
  (set `self.AliveMI` _returnvalue_2)
  (`self.AliveRoll`)
  (`KismetSystemLibrary.K2_SetTimer` null "CheckNeighbours" 0.5 true 2.0))

(event `CheckNeighbours`
  (bind _returnvalue (`self.K2_GetActorLocation`))
  (bind _alivecellneighborcounter (`self.AliveCellNeighborCounter`))
  (for _ (range 8)
    (bind (_outhit _returnvalue_2) (`KismetSystemLibrary.LineTraceSingle` :`Start` _returnvalue :`End` (+ _returnvalue (* (`KismetMathLibrary.GreaterGreater_VectorRotator` (`self.GetActorForwardVector`) (`KismetMathLibrary.MakeRotator` 0.0 0.0 (`self.RotateLineTrace`))) 200.0)) :`TraceChannel` "TraceTypeQuery1" :`DrawDebugType` "Persistent"))
    (if _returnvalue_2
      (bind _asbp_cell (cast `/Game/Blueprints/GameOfLifeBP/BP_Cell` (`.HitActor` (`GameplayStatics.BreakHitResult` _outhit)))
        (:`then`
          (if (`/Game/Blueprints/GameOfLifeBP/BP_Cell.IsAlive` _asbp_cell)
            (`/Engine/EditorBlueprintResources/StandardMacros.IncrementInt` (`self.AliveCellNeighborCounter`)
              (:`  `
                _))))
        (:`CastFailed`
          _)))
    (set `self.RotateLineTrace` (+ (`self.RotateLineTrace`) 45.0)))
  (if (or (== _alivecellneighborcounter 2) (== _alivecellneighborcounter 3))
    (`self.SetCellAlive`)
    (else
      (`self.SetCellDead`))))

(event `SetCellAlive`
  (set `self.IsAlive` true)
  (`PrimitiveComponent.SetMaterial` (`self.Cell`) 0 (`self.AliveMI`) :!label _label)
  (bind (_direction _0_1hueline) (`Timeline|CycleHue`)
    (:`Update`
      (`MaterialInstanceDynamic.SetScalarParameterValue` (`self.AliveMI`) "CellBaseColorHue" _0_1hueline))))

(event `SetCellDead`
  (set `self.IsAlive` false)
  (`PrimitiveComponent.SetMaterial` (`self.Cell`) 0 (`self.DeadMI`) :!label _label_2)
  (bind (_direction _0_1valueline) (`Timeline|CycleValue`)
    (:`Update`
      (`MaterialInstanceDynamic.SetScalarParameterValue` (`self.DeadMI`) "CellBaseColorValue" _0_1valueline))))

(event `AliveRoll`
  (bind _output_get (set `self.IsAlive` (`KismetMathLibrary.RandomBool`)))
  (if _output_get
    (goto _label)
    (else
      (goto _label_2))))

(fn `OnRep_IsAlive`)

(fn `UserConstructionScript`)