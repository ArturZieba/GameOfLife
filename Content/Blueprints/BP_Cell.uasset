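; BP_Cell is a grid cell for a Game of Life-style simulation that starts randomly alive or dead.
; A looping one-second timer line-traces around the cell in 45-degree steps to count living BP_Cell neighbours.
; A count of 2 or 3 makes it alive and other counts up to 8 kill it, with timelines applying the matching material.
; The neighbour counter is never reset between checks.
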(event `self.ReceiveBeginPlay`
  (`self.AliveRoll`)
  (`KismetSystemLibrary.K2_SetTimer` null "CheckNeighbours" 1.0 true 1.0))

(event `CheckNeighbours`
  (bind _returnvalue (`self.K2_GetActorLocation`))
  (for _ (range 9)
    (bind (_outhit _returnvalue_2) (`KismetSystemLibrary.LineTraceSingle` _returnvalue (+ _returnvalue (* (`KismetMathLibrary.GreaterGreater_VectorRotator` (`self.GetActorForwardVector`) (`KismetMathLibrary.MakeRotator` 0.0 0.0 (`self.RotateLineTrace`))) 200.0)) "TraceTypeQuery1"))
    (if _returnvalue_2
      (bind _asbp_cell (cast `/Game/Blueprints/BP_Cell` (`.HitActor` (`GameplayStatics.BreakHitResult` _outhit))))
      (if (`/Game/Blueprints/BP_Cell.IsAlive` _asbp_cell)
        (`/Engine/EditorBlueprintResources/StandardMacros.IncrementInt` (`self.AliveCellNeighborCounter`)
          (:`  `
            _))))
    (set `self.RotateLineTrace` (+ (`self.RotateLineTrace`) 45.0)))
  (switch `int` (`self.AliveCellNeighborCounter`)
    (:`0`
      (`self.SetCellDead` :!label _label))
    (:`1`
      (goto _label))
    (:`2`
      (`self.SetCellAlive` :!label _label_2))
    (:`3`
      (goto _label_2))
    (:`4`
      (goto _label))
    (:`5`
      (goto _label))
    (:`6`
      (goto _label))
    (:`7`
      (goto _label))
    (:`8`
      (goto _label))))

(event `SetCellAlive`
  (set `self.IsAlive` true)
  (bind (_direction _0_1hueline) (`Timeline|CycleHue` :!label _label_3)
    (:`Update`
      (`PrimitiveComponent.SetMaterial` (`self.Cell`) 0 "/Game/Materials/M_CellAlive.M_CellAlive"))))

(event `SetCellDead`
  (set `self.IsAlive` false)
  (bind (_direction _0_1hueline) (`Timeline|Timeline` :!label _label_4)
    (:`Update`
      (`PrimitiveComponent.SetMaterial` (`self.Cell`) 0 "/Game/Materials/M_CellDead.M_CellDead"))))

(event `AliveRoll`
  (bind _output_get (set `self.IsAlive` (`KismetMathLibrary.RandomBool`)))
  (if _output_get
    (goto _label_3)
    (else
      (goto _label_4))))

(event `self.ReceiveTick`
  (params (DeltaSeconds :type "Float (single-precision)")))

(fn `OnRep_IsAlive`)

(fn `UserConstructionScript`)